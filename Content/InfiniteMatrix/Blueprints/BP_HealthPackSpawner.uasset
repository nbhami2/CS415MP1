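; BP_HealthPackSpawner is a Blueprint that spawns a health pack pickup ahead of the player along the X axis.
; On BeginPlay it calls SpawnHealthPacks once, which spawns a BP_HealthPack at a fixed offset from player pawn 0's X position, with Y and Z at zero, and prints a debug message.
; Random offset nodes are present in the function but unused, so placement is not randomized.
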(event `self.ReceiveBeginPlay`
  (`self.SpawnHealthPacks`))

(fn `SpawnHealthPacks`
  (bind _returnvalue_x (`KismetMathLibrary.BreakVector` (`self.K2_GetActorLocation` (`GameplayStatics.GetPlayerPawn` 0))))
  (`|SpawnActorFromClass` "/Game/InfiniteMatrix/Blueprints/BP_HealthPack.BP_HealthPack_C" (`KismetMathLibrary.MakeTransform` (`KismetMathLibrary.MakeVector` (+ 2000.0 _returnvalue_x))) "Undefined" "MultiplyWithRoot" null null)
  (`KismetSystemLibrary.PrintString` "spawned"))

(fn `UserConstructionScript`)