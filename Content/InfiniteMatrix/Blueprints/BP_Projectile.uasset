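; BP_Projectile is a projectile that destroys enemies it hits and is meant to award score to the player.
; Its sphere's hit event ignores BP_Player, destroys any BP_Enemy, and destroys the projectile on every non-player hit.
; The score increment uses the player reference from the failed cast, so it has no valid target.
; Tick raises ProjectileVelocity by a fixed amount each frame, independent of delta time.
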(event `self.ReceiveTick`
  (params (DeltaSeconds :type "Float (single-precision)"))
  (set `self.ProjectileVelocity` (+ 1.0 (`self.ProjectileVelocity`))))

(event `self.Sphere.OnComponentHit`
  (params (HitComponent :type "PrimitiveComponent Object Reference") (OtherActor :type "Actor Object Reference") (OtherComp :type "PrimitiveComponent Object Reference") (NormalImpulse :type "Vector Structure") (Hit :type "HitResult Structure (by ref)"))
  (bind _asbp_player (cast `/Game/InfiniteMatrix/Blueprints/BP_Player` OtherActor)
    (:`CastFailed`
      (bind _asbp_enemy (cast `/Game/InfiniteMatrix/Blueprints/BP_Enemy` OtherActor)
        (:`then`
          (bind _result (`/Engine/EditorBlueprintResources/StandardMacros.IncrementInt` (`/Game/InfiniteMatrix/Blueprints/BP_Player.Score` _asbp_player))
            (:`  `
              (set `/Game/InfiniteMatrix/Blueprints/BP_Player.Score` _result _asbp_player)
              (`self.K2_DestroyActor` _asbp_enemy))))
        (:`CastFailed`
          _))
      (`self.K2_DestroyActor`))))

(fn `UserConstructionScript`)