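; BP_HealthPack is a health pickup that restores a small fixed amount of health to BP_Player on overlap.
; Tick spins the Cube mesh around yaw at a rate set by HealthRotate.
; On overlap it adds health, clamped at the maximum, if the player is below full.
; It then destroys its Cube, Cube1 and Box components even at full health, without destroying the actor itself.
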(event `self.ReceiveTick`
  (params (DeltaSeconds :type "Float (single-precision)"))
  (`SceneComponent.K2_AddLocalRotation` (`self.Cube`) (`KismetMathLibrary.MakeRotator` 0.0 0.0 (* DeltaSeconds (`self.HealthRotate`))) false false))

(event `self.ReceiveActorBeginOverlap`
  (params (OtherActor :type "Actor Object Reference"))
  (bind _asbp_player (cast `/Game/InfiniteMatrix/Blueprints/BP_Player` OtherActor))
  (if (< (`/Game/InfiniteMatrix/Blueprints/BP_Player.CurrentHealth` _asbp_player) 100.0)
    (set `/Game/InfiniteMatrix/Blueprints/BP_Player.CurrentHealth` (`KismetMathLibrary.FClamp` (+ (`/Game/InfiniteMatrix/Blueprints/BP_Player.CurrentHealth` _asbp_player) 5.0) 0.0 100.0) _asbp_player))
  (`ActorComponent.K2_DestroyComponent` (`self.Cube1`))
  (`ActorComponent.K2_DestroyComponent` (`self.Cube`))
  (`ActorComponent.K2_DestroyComponent` (`self.Box`)))

(fn `UserConstructionScript`)